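; PumpkinGrenade is a thrown grenade actor that launches, explodes visually after a fixed fuse, then removes itself.
; Shoot applies a velocity-change impulse to the mesh, forward and upward scaled by ShootLevel, at world origin, and starts a named timer for Explode.
; Explode spawns an attached particle system and binds its finished event, apparently to Die, which destroys the actor.
; The file contains no damage logic.
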(event EventBeginPlay)

(event Collision|EventActorBeginOverlap
  (params (OtherActor :type Actor%20Object%20Reference)))

(event EventTick
  (params (DeltaSeconds :type Float%20%28single-precision%29)))

(fn ConstructionScript)

(fn Explode
  (bind _returnvalue (Niagara|SpawnSystemAttached (LocalVariables|GetExplosionParticle) (Variables|Default|GetStaticMesh) "None" "0, 0, 0" "0, 0, 0" "KeepRelativeOffset" false))
  (EventDispatchers|BindEventtoOnSystemFinished _returnvalue (EventDispatchers|CreateEvent :!event Die)))

(fn Die
  (params (PSystem :type Niagara%20Component%20Object%20Reference))
  (Actor|DestroyActor))

(fn Shoot
  (params (ShootLevel :type Integer))
  (bind _returnvalue (Math|Conversions|ToFloat(Integer) ShootLevel))
  (bind _returnvalue_2 (* _returnvalue 2e+02))
  (Class|PrimitiveComponent|AddVelocityChangeImpulseatLocation (Variables|Default|GetStaticMesh) (+ (* (Transformation|GetActorForwardVector) (Math|Vector|MakeVector _returnvalue_2 _returnvalue_2 0.0)) (Math|Vector|MakeVector 0.0 0.0 _returnvalue_2)) "0, 0, 0" "None")
  (Utilities|Time|SetTimerbyFunctionName 0 "Explode" 3.0))