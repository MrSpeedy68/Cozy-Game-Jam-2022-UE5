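; BP_HealthPotion is a health pickup that spins in place until a player collects it.
; On overlap with BP_ThirdPersonCharacter it adds HealthAmount to the character's health, with no clamp applied here.
; It then passes health, energy and pumpkin count to the character's OnUpdateUI and destroys itself.
; Tick applies a frame-rate-independent yaw rotation for the spin.
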(event EventBeginPlay)

(event Collision|EventActorBeginOverlap
  (params (OtherActor :type Actor%20Object%20Reference))
  (bind _asbp_third_person_character (Utilities|Casting|CastToBP_ThirdPersonCharacter OtherActor))
  (bind _output_get (Variables|Default|SetPlayer _asbp_third_person_character))
  (Class|FallGameJam2022Character|SetHealth _output_get (+ (Class|FallGameJam2022Character|GetHealth (Variables|Default|GetPlayer)) (Variables|Default|GetHealthAmount)))
  (Default|OnUpdateUI (Variables|Default|GetPlayer) (Class|FallGameJam2022Character|GetHealth (Variables|Default|GetPlayer)) (Class|FallGameJam2022Character|GetEnergy (Variables|Default|GetPlayer)) (.pumpkins (Class|FallGameJam2022Character|GetInventory (Variables|Default|GetPlayer))))
  (Actor|DestroyActor))

(event EventTick
  (params (DeltaSeconds :type Float%20%28single-precision%29))
  (Transformation|SetActorRotation (Math|Transform|TransformRotation (Transformation|GetActorTransform) (Math|Rotator|MakeRotator 0.0 0.0 (* DeltaSeconds 45.0)))))

(fn ConstructionScript)