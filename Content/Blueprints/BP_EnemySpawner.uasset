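; BP_EnemySpawner is an enemy spawner that tops up the level's BP_EnemyAI population at its own location.
; Tick counts all BP_EnemyAI actors and, below a fixed cap, passes through a Delay that spaces out SpawnAIFromClass calls, without rechecking the count afterward.
; A separate TrySpawn function spawns and stores a single EnemyActor when that reference is invalid, but nothing in this Blueprint calls it.
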(event EventBeginPlay)

(event Collision|EventActorBeginOverlap
  (params (OtherActor :type Actor%20Object%20Reference)))

(event EventTick
  (params (DeltaSeconds :type Float%20%28single-precision%29))
  (bind _outactors (Actor|GetAllActorsOfClass "/Game/Blueprints/BP_EnemyAI.BP_EnemyAI_C"))
  (if (< (Utilities|Array|Length _outactors) 10)
    (Utilities|FlowControl|Delay 3.0)
    (AI|SpawnAIFromClass "/Game/Blueprints/BP_EnemyAI.BP_EnemyAI_C" 0 (Transformation|GetActorLocation) "0, 0, 0" false 0)))

(fn ConstructionScript)

(fn TrySpawn
  (if (not (Utilities|IsValid (Variables|Default|GetEnemyActor)))
    (bind _returnvalue (Game|SpawnActorfromClass "/Game/Blueprints/BP_EnemyAI.BP_EnemyAI_C" (Math|Conversions|ToTransform(Vector) (Transformation|GetActorLocation self)) "Undefined" 0 0))
    (Variables|Default|SetEnemyActor _returnvalue)))