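; BP_Spawner is a spawner actor that keeps a single pumpkin present at its location.
; On BeginPlay it starts a looping timer at the TimeToSpawn interval that calls TrySpawn.
; TrySpawn spawns a BP_Pumpkin only when the stored Pumpkin reference is no longer valid, so a replacement appears on a later tick of the timer after the previous one is destroyed.
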(event EventBeginPlay
  (Utilities|Time|SetTimerbyFunctionName 0 "TrySpawn" (Variables|Default|GetTimeToSpawn) true))

(event Collision|EventActorBeginOverlap
  (params (OtherActor :type Actor%20Object%20Reference)))

(event EventTick
  (params (DeltaSeconds :type Float%20%28single-precision%29)))

(fn ConstructionScript)

(fn TrySpawn
  (if (not (Utilities|IsValid (Variables|Default|GetPumpkin)))
    (bind _returnvalue (Game|SpawnActorfromClass "/Game/Blueprints/BP_Pumpkin.BP_Pumpkin_C" (Math|Conversions|ToTransform(Vector) (Transformation|GetActorLocation self)) "Undefined" 0 0))
    (Variables|Default|SetPumpkin _returnvalue)))