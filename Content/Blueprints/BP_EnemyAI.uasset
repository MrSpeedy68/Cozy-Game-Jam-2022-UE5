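; Enemy AI character that chases the player, deals contact-range damage and can be killed with pumpkin grenades.
; Pawn sensing latches a seen flag, never effectively cleared, and starts an AI MoveTo toward the player.
; Tick applies tiny damage every frame while the living enemy is within attack distance, halting movement if it has not seen the player.
; Only BP_PumpkinGrenade damage reduces health; death stops movement and starts a timed despawn.
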(event OnSeePawn(PawnSensing)
  (params (Pawn :type Pawn%20Object%20Reference))
  ;[0.403 0.5311 1] Follow Player
  (if (not (Variables|Default|GetIsDead?))
    (Variables|Default|SetIsSeeingPlayer? true)
    (CallFunction|FollowPlayer)))

(event Custom|FollowPlayer
  ;[0.403 0.5311 1] Follow Player
  (if (Variables|Default|GetIsSeeingPlayer?)
    (AI|AIMoveTo self "0, 0, 0" (Game|GetPlayerCharacter 0) 7e+01 false)
    (else
      (Variables|Default|SetIsSeeingPlayer? false))))

(event Custom|Despawn
  ;[1 0.1264 0.2462] Take Damage
  (Actor|DestroyActor))

(event EventBeginPlay)

(event Collision|EventActorBeginOverlap
  (params (OtherActor :type Actor%20Object%20Reference)))

(event EventTick
  (params (DeltaSeconds :type Float%20%28single-precision%29))
  (bind _returnvalue (Game|GetPlayerCharacter 0))
  ;[1 0.3642 0.735] Check if can attack
  (bind _output_get (Variables|Default|SetCanAttack? (<= (Math|Vector|Distance(Vector) (Transformation|GetActorLocation) (Transformation|GetActorLocation _returnvalue)) (Variables|Default|GetAttackDistance))))
  (if (and _output_get (not (Variables|Default|GetIsDead?)))
    (Game|Damage|ApplyDamage _returnvalue 0.001 0 self)
    (if (not (Variables|Default|GetIsSeeingPlayer?))
      (Components|Movement|StopMovementImmediately (Variables|Character|GetCharacterMovement)))))

(event Game|Damage|EventAnyDamage
  (params (Damage :type Float%20%28single-precision%29) (DamageType :type Damage%20Type%20Object%20Reference) (InstigatedBy :type Controller%20Object%20Reference) (DamageCauser :type Actor%20Object%20Reference))
  ;[1 0.1264 0.2462] Take Damage
  (Utilities|Casting|CastToBP_PumpkinGrenade DamageCauser)
  (bind _output_get (Variables|Default|SetMonster%20Health (- (Variables|Default|GetMonster%20Health) Damage)))
  (Variables|Default|SetIsDead? (<= _output_get 0.0))
  (if (Variables|Default|GetIsDead?)
    (Components|Movement|StopMovementImmediately (Variables|Character|GetCharacterMovement))
    (Utilities|Time|SetTimerbyEvent (delegate Custom|Despawn) (Variables|Default|GetDespawn%20Time))))

(fn ConstructionScript)