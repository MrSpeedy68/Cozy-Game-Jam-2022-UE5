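; Pumpkin grenade actor that is launched and explodes on a timer, dealing radial damage.
; Shoot applies a forward and upward velocity impulse to the mesh, scaled by ShootLevel, then starts a three-second timer for Explode.
; Explode spawns an attached particle system and scales damage and radius by the player character's DamageLevel and BlastRadiusLevel stats.
; A callback on the particle system finishing, apparently Die, destroys the actor.
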(event EventBeginPlay)

(event Collision|EventActorBeginOverlap
  (params (OtherActor :type Actor%20Object%20Reference)))

(event EventTick
  (params (DeltaSeconds :type Float%20%28single-precision%29)))

(fn ConstructionScript)

(fn Explode
  (bind _returnvalue (Niagara|SpawnSystemAttached (LocalVariables|GetExplosionParticle) (Variables|Default|GetStaticMesh) "None" "0, 0, 0" "0, 0, 0" "KeepRelativeOffset" false))
  (EventDispatchers|BindEventtoOnSystemFinished _returnvalue (EventDispatchers|CreateEvent :!event Die))
  (bind _asbp_third_person_character (Utilities|Casting|CastToBP_ThirdPersonCharacter (Game|GetPlayerCharacter 0)))
  (Game|Damage|ApplyRadialDamage (* (.damagelevel (Class|FallGameJam2022Character|GetPlayerStats _asbp_third_person_character)) (Variables|Default|GetBase%20Damage)) (Transformation|GetActorLocation) (* (.blastradiuslevel (Class|FallGameJam2022Character|GetPlayerStats _asbp_third_person_character)) (Variables|Default|GetBlast%20Radius)) 0 0 self 0 false "ECC_WorldStatic"))

(fn Die
  (params (PSystem :type Niagara%20Component%20Object%20Reference))
  (Actor|DestroyActor))

(fn Shoot
  (params (ShootLevel :type Integer))
  (bind _returnvalue (Math|Conversions|ToFloat(Integer) ShootLevel))
  (bind _returnvalue_2 (* _returnvalue 2e+02))
  (Class|PrimitiveComponent|AddVelocityChangeImpulseatLocation (Variables|Default|GetStaticMesh) (+ (* (Transformation|GetActorForwardVector) (Math|Vector|MakeVector _returnvalue_2 _returnvalue_2 0.0)) (Math|Vector|MakeVector 0.0 0.0 _returnvalue_2)) "0, 0, 0" "None")
  (Utilities|Time|SetTimerbyFunctionName 0 "Explode" 3.0))